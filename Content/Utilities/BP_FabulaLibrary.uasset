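; Blueprint function library that computes damage for the Fabula combat rules using GAS attributes and gameplay tags.
; CalculateDamage adds HR to the source's weapon damage attribute, subtracts a target attribute (RD) and scales the result by an affinity multiplier.
; GetAffinityDamageMultiplier switches on the damage type tag to pick that element's affinity tags.
; GetEffectiveDamageAffility resolves them by priority: absorption negates the sign, immunity zeroes, and resistance and vulnerability cancel out.
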(fn CalculateDamage
  (params (HR :type Float%20%28double-precision%29) (Source :type Fabula%20Ability%20System%20Component%20Object%20Reference) (WeaponDamage :type Gameplay%20Attribute%20Structure) (DamageType :type Gameplay%20Tag%20Structure) (Target :type Fabula%20Ability%20System%20Component%20Object%20Reference))
  (return (|(((HR+base)-RD)*Mult) HR (.ReturnValue (Class|AbilitySystemComponent|GetGameplayAttributeValue Source WeaponDamage)) (.ReturnValue (Class|AbilitySystemComponent|GetGameplayAttributeValue Target "(AttributeName=\"DamageReduction\",Attribute=/Script/GASExercise.FabulaAttributeSet:DamageReduction,AttributeOwner=\"/Script/CoreUObject.Class'/Script/GASExercise.FabulaAttributeSet'\")")) (CallFunction|GetAffinityDamageMultiplier DamageType Target Target))))

(fn GetAffinityDamageMultiplier
  (params (DamageType :type Gameplay%20Tag%20Structure) (Target :type Fabula%20Ability%20System%20Component%20Object%20Reference))
  ;[1 1 1] This awful structure is by itself argument against using GAS
  (|SwitchGameplayTag DamageType
    (:Default
      (Development|PrintString Target "UNKNOWN DAMAGE TYPE")
      (return 1.0))
    (:Fabula.DamageType.Air
      (return (CallFunction|GetEffectiveDamageAffility Target "(TagName=\"Fabula.Affinity.Air.Absorption\")" "(TagName=\"Fabula.Affinity.Air.Immunity\")" "(TagName=\"Fabula.Affinity.Air.Resistance\")" "(TagName=\"Fabula.Affinity.Air.Vulnerability\")" Target)))
    (:Fabula.DamageType.Bolt
      (return (CallFunction|GetEffectiveDamageAffility Target "(TagName=\"Fabula.Affinity.Bolt.Absorption\")" "(TagName=\"Fabula.Affinity.Bolt.Immunity\")" "(TagName=\"Fabula.Affinity.Bolt.Resistance\")" "(TagName=\"Fabula.Affinity.Bolt.Vulnerability\")" Target)))
    (:Fabula.DamageType.Dark
      (return (CallFunction|GetEffectiveDamageAffility Target "(TagName=\"Fabula.Affinity.Dark.Absorption\")" "(TagName=\"Fabula.Affinity.Dark.Immunity\")" "(TagName=\"Fabula.Affinity.Dark.Resistance\")" "(TagName=\"Fabula.Affinity.Dark.Vulnerability\")" Target)))
    (:Fabula.DamageType.Earth
      (return (CallFunction|GetEffectiveDamageAffility Target "(TagName=\"Fabula.Affinity.Earth.Absorption\")" "(TagName=\"Fabula.Affinity.Earth.Immunity\")" "(TagName=\"Fabula.Affinity.Earth.Resistance\")" "(TagName=\"Fabula.Affinity.Earth.Vulnerability\")" Target)))
    (:Fabula.DamageType.Fire
      (return (CallFunction|GetEffectiveDamageAffility Target "(TagName=\"Fabula.Affinity.Fire.Absorption\")" "(TagName=\"Fabula.Affinity.Fire.Immunity\")" "(TagName=\"Fabula.Affinity.Fire.Resistance\")" "(TagName=\"Fabula.Affinity.Fire.Vulnerability\")" Target)))
    (:Fabula.DamageType.Ice
      (return (CallFunction|GetEffectiveDamageAffility Target "(TagName=\"Fabula.Affinity.Ice.Absorption\")" "(TagName=\"Fabula.Affinity.Ice.Immunity\")" "(TagName=\"Fabula.Affinity.Ice.Resistance\")" "(TagName=\"Fabula.Affinity.Ice.Vulnerability\")" Target)))
    (:Fabula.DamageType.Light
      (return (CallFunction|GetEffectiveDamageAffility Target "(TagName=\"Fabula.Affinity.Light.Absorption\")" "(TagName=\"Fabula.Affinity.Light.Immunity\")" "(TagName=\"Fabula.Affinity.Light.Resistance\")" "(TagName=\"Fabula.Affinity.Light.Vulnerability\")" Target)))
    (:Fabula.DamageType.Phys
      (return (CallFunction|GetEffectiveDamageAffility Target "(TagName=\"Fabula.Affinity.Phys.Absorption\")" "(TagName=\"Fabula.Affinity.Phys.Immunity\")" "(TagName=\"Fabula.Affinity.Phys.Resistance\")" "(TagName=\"Fabula.Affinity.Phys.Vulnerability\")" Target)))
    (:Fabula.DamageType.Poison
      (return (CallFunction|GetEffectiveDamageAffility Target "(TagName=\"Fabula.Affinity.Poison.Absorption\")" "(TagName=\"Fabula.Affinity.Poison.Immunity\")" "(TagName=\"Fabula.Affinity.Poison.Resistance\")" "(TagName=\"Fabula.Affinity.Poison.Vulnerability\")" Target)))))

(fn GetEffectiveDamageAffility
  (params (FabulaComponent :type Fabula%20Ability%20System%20Component%20Object%20Reference) (Absorption :type Gameplay%20Tag%20Structure) (Immunity :type Gameplay%20Tag%20Structure) (Resistance :type Gameplay%20Tag%20Structure) (Vulnerability :type Gameplay%20Tag%20Structure))
  (bind _returnvalue (GameplayTags|HasMatchingGameplayTag FabulaComponent Vulnerability))
  (bind _returnvalue_2 (GameplayTags|HasMatchingGameplayTag FabulaComponent Resistance))
  (if (GameplayTags|HasMatchingGameplayTag FabulaComponent Absorption)
    (return -1.0)
    (elif (GameplayTags|HasMatchingGameplayTag FabulaComponent Immunity)
      (return 0.0)
      (elif (and _returnvalue_2 _returnvalue)
        (return 1.0)
        (elif _returnvalue_2
          (return 0.5)
          (elif _returnvalue
            (return 2.0)
            (else
              (return 1.0))))))))