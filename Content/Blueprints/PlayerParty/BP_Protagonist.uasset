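; Player party protagonist character that brings its companion into the level.
; On BeginPlay it spawns a BP_Companion at its own transform, sets itself as commander and adds the companion's ability system component to its party.
; A TODO marks this spawning as a candidate to move higher, possibly into a Subsystem.
; When unpossessed, it stops character movement immediately.
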(event EventBeginPlay
  (|CallParentFunction)
  ;[1 1 1] TODO: this logic should be executed somewhere higher, maybe by Subsystem, that is called instead of default Character Spawn on level loaded
  (bind _returnvalue (Game|SpawnActorfromClass "/Game/Blueprints/PlayerParty/BP_Companion.BP_Companion_C" (Transformation|GetActorTransform) "AdjustIfPossibleButAlwaysSpawn" "MultiplyWithRoot" 0 0))
  (Default|SetCommander _returnvalue self)
  (Class|FabulaParty|AddCreature (Class|FabulaAbilitySystemComponent|GetParty (Variables|Default|GetAbilitySystemComp)) (Class|FabulaCharacter|GetAbilitySystemComponent _returnvalue)))

(event EventUnpossessed
  (params (OldController :type Controller%20Object%20Reference))
  ;[1 1 1] Just to be sure
  (Components|Movement|StopMovementImmediately (Variables|Character|GetCharacterMovement)))

(event EventTick
  (params (DeltaSeconds :type Float%20%28single-precision%29))
  (|CallParentFunction DeltaSeconds) ; This node is disabled and will not be called.\nDrag off pins to build functionality.
)

(event Collision|EventActorBeginOverlap
  (params (OtherActor :type Actor%20Object%20Reference)))

(fn ConstructionScript
  (|CallParentFunction))