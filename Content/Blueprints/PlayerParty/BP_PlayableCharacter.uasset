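; Playable party character built on GAS with a Fabula attribute set, used in round-based combat.
; BeginPlay registers attributes with its card widget, grants a damage ability, applies initial stats and spawns a party containing itself.
; Ability component events halt movement and AI logic when combat starts, reset turns each round unless dead, and shift the camera over the shoulder for targeting.
; Reaching zero HP applies a death effect and ragdolls the mesh.
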(event OnRoundStarted(AbilitySystemComp)
  (bind _abilitysystemcomp (Variables|Default|GetAbilitySystemComp))
  (if (not (GameplayTags|HasMatchingGameplayTag _abilitysystemcomp "(TagName=\"Fabula.Status.Dead\")"))
    (GameplayEffects|ApplyGameplayEffectToSelf :self _abilitysystemcomp :GameplayEffectClass "/Game/Effects/GE_ResetTurns.GE_ResetTurns_C")))

(event OnCombatStarted(AbilitySystemComp)
  (bind _returnvalue (Pawn|GetController))
  (Components|Movement|StopMovementImmediately (Variables|Character|GetCharacterMovement))
  (Utilities|IsValid _returnvalue
    (:Is%20Valid
      (AI|Navigation|StopMovement _returnvalue)
      (bind _asaicontroller (Utilities|Casting|CastToAIController _returnvalue))
      (AI|Logic|StopLogic (Variables|/Script/AIModule.AIController|GetBrainComponent _asaicontroller) ""))))

(event OnTargettingModeActivated(AbilitySystemComp)
  (bind _cameraboom (Variables|Default|GetCameraBoom))
  (Transformation|SetRelativeLocation _cameraboom "0.000000,0.000000,70.000000" false false)
  (Variables|/Script/Engine.SpringArmComponent|SetTargetArmLength _cameraboom 3e+01)
  (Variables|/Script/Engine.SpringArmComponent|SetSocketOffset _cameraboom "0.000000,30.000000,0.000000"))

(event OnTargettingModeDeactivated(AbilitySystemComp)
  (bind _cameraboom (Variables|Default|GetCameraBoom))
  (Transformation|SetRelativeLocation _cameraboom "0, 0, 0" false false)
  (Variables|/Script/Engine.SpringArmComponent|SetTargetArmLength _cameraboom 4e+02)
  (Variables|/Script/Engine.SpringArmComponent|SetSocketOffset _cameraboom "0.000000,0.000000,0.000000"))

(event Custom|OnKilled
  (bind _mesh (Variables|Character|GetMesh))
  (GameplayEffects|ApplyGameplayEffectToSelf :self (Variables|Default|GetAbilitySystemComp) :GameplayEffectClass "/Game/Effects/GE_Death.GE_Death_C")
  ;[1 1 1] This one should react to getting tag, not JUST reaching zero HP. Yes, at this point my patience for GAS reached boiling point
  (Physics|SetSimulatePhysics _mesh true)
  (Collision|SetCollisionProfileName _mesh "Ragdoll" true :!class /Script/Engine.PrimitiveComponent))

(event EventBeginPlay
  (Default|RegisterAttributes (.AsWBP%20Creature%20Card%20Simplified (Utilities|Casting|CastToWBP_CreatureCardSimplified (UserInterface|GetWidget (Variables|Default|GetWidget)))) (Variables|Default|GetAttributeSet))
  (GameplayAbilities|GiveAbility (Variables|Default|GetAbilitySystemComp) "/Game/Abilities/GA_DealDamage.GA_DealDamage_C" 0 -1)
  (GameplayEffects|ApplyGameplayEffectToSelf :self (Variables|Default|GetAbilitySystemComp) :GameplayEffectClass (Variables|Default|GetInitData))
  (bind _returnvalue (GameplayAttributes|GetAttributeSet (Variables|Default|GetAbilitySystemComp) "/Script/GASExercise.FabulaAttributeSet"))
  (bind _asfabula_attribute_set (Utilities|Casting|CastToFabulaAttributeSet _returnvalue))
  (EventDispatchers|BindEventtoOnHPReachedZero _asfabula_attribute_set (delegate Custom|OnKilled))
  (bind _returnvalue_2 (Game|SpawnActorfromClass "/Game/Blueprints/BP_Party.BP_Party_C" (Transformation|GetActorTransform) "Undefined" "MultiplyWithRoot" 0 0))
  (Class|FabulaParty|AddCreature _returnvalue_2 (Variables|Default|GetAbilitySystemComp)))

(event EventTick
  (params (DeltaSeconds :type Float%20%28single-precision%29)))

(fn ConstructionScript)

(fn SetCommander
  (params (InCommander :type Actor%20Object%20Reference)))