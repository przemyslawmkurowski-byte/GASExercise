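; Player pawn for JRPG turn-based combat that drives character, skill and target selection.
; On possession it creates the combat menu and a circular, dead-skipping iterator over the player party.
; Each selection stage swaps Enhanced Input mapping contexts, with the camera following character selection and chosen skills activating as abilities.
; Target requests return the caster or a chosen enemy through a stored callback, yawing the caster toward the highlighted enemy.
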(event Custom|StartCombat
  (bind _returnvalue (UserInterface|CreateWidget "/Game/UI/WBP_CombatMenu.WBP_CombatMenu_C" (.AsPlayer%20Controller (Utilities|Casting|CastToPlayerController (Pawn|GetController))) self))
  (UserInterface|Viewport|AddtoViewport _returnvalue 0)
  (Variables|Default|SetCombatMenu _returnvalue)
  (bind _output_get (Variables|Default|SetPlayerParty (Class|GlobalActorSubsystem|GetPlayerParty (Subsystems|GetGlobalActorSubsystem))))
  (bind _returnvalue_2 (Class|FabulaParty|GetIterator _output_get (Utilities|Struct|MakeFabulaPartyIteratorPolicy true true)))
  (Variables|Default|SetSelfPartyIterator _returnvalue_2))

(event Input|EnhancedActionEvents|EnhancedInputActionIA_PrevCharacter
  (params (ActionValue :type Boolean) (ElapsedSeconds :type Float%20%28double-precision%29) (TriggeredSeconds :type Float%20%28double-precision%29) (InputAction :type Input%20Action%20Object%20Reference :default "/Game/Input/Combat/IA_PrevCharacter.IA_PrevCharacter"))
  ;[1 1 1] Select character
  (bind _returnvalue (Class|FabulaPartyIteratorLibrary|Prev (Variables|Default|GetSelfPartyIterator)))
  (Game|Player|SetViewTargetwithBlend (Variables|Default|GetCachedPlayerController) (Components|GetOwner _returnvalue) 0.25 "VTBlend_Linear" 0.0 false))

(event Input|EnhancedActionEvents|EnhancedInputActionIA_NextCharacter
  (params (ActionValue :type Boolean) (ElapsedSeconds :type Float%20%28double-precision%29) (TriggeredSeconds :type Float%20%28double-precision%29) (InputAction :type Input%20Action%20Object%20Reference :default "/Game/Input/Combat/IA_NextCharacter.IA_NextCharacter"))
  ;[1 1 1] Select character
  (bind _returnvalue (Class|FabulaPartyIteratorLibrary|Next (Variables|Default|GetSelfPartyIterator)))
  (Game|Player|SetViewTargetwithBlend (Variables|Default|GetCachedPlayerController) (Components|GetOwner _returnvalue) 0.25 "VTBlend_Linear" 0.0 false))

(event Input|EnhancedActionEvents|EnhancedInputActionIA_SelectCharacter
  (params (ActionValue :type Boolean) (ElapsedSeconds :type Float%20%28double-precision%29) (TriggeredSeconds :type Float%20%28double-precision%29) (InputAction :type Input%20Action%20Object%20Reference :default "/Game/Input/Combat/IA_SelectCharacter.IA_SelectCharacter"))
  (bind _cachedplayercontroller (Variables|Default|GetCachedPlayerController))
  (bind _returnvalue (PlayerController|LocalPlayerSubsystems|GetEnhancedInputLocalPlayerSubsystem _cachedplayercontroller))
  ;[1 1 1] Select character
  (bind _returnvalue_2 (Class|FabulaPartyIteratorLibrary|TryGetCurrent (Variables|Default|GetSelfPartyIterator)))
  (if (Class|FabulaAbilitySystemComponent|HasTurns _returnvalue_2)
    (Class|EnhancedInputSubsystemInterface|ClearAllMappings _returnvalue)
    (Input|AddMappingContext _returnvalue "/Game/Input/Combat/IMC_SkillSelect.IMC_SkillSelect" 0 "(bIgnoreAllPressedKeysUntilRelease=True,bForceImmediately=False,bNotifyUserSettings=False)")
    (bind _returnvalue_3 (Class|FabulaPartyIteratorLibrary|TryGetCurrent (Variables|Default|GetSelfPartyIterator)))
    (bind _outwidget (Default|OpenAbilitySelection (Variables|Default|GetCombatMenu) _returnvalue_3))
    (Variables|Default|SetActionSelector _outwidget)
    (else
      (Development|PrintString "Cannot select Creature that doesn't have turns"))))

(event Input|EnhancedActionEvents|EnhancedInputActionIA_PrevSkill
  (params (ActionValue :type Boolean) (ElapsedSeconds :type Float%20%28double-precision%29) (TriggeredSeconds :type Float%20%28double-precision%29) (InputAction :type Input%20Action%20Object%20Reference :default "/Game/Input/Combat/IA_PrevSkill.IA_PrevSkill"))
  ;[1 1 1] Select skill
  (Default|Prev (Variables|Default|GetActionSelector)))

(event Input|EnhancedActionEvents|EnhancedInputActionIA_NextSkill
  (params (ActionValue :type Boolean) (ElapsedSeconds :type Float%20%28double-precision%29) (TriggeredSeconds :type Float%20%28double-precision%29) (InputAction :type Input%20Action%20Object%20Reference :default "/Game/Input/Combat/IA_NextSkill.IA_NextSkill"))
  ;[1 1 1] Select skill
  (Default|Next (Variables|Default|GetActionSelector)))

(event Input|EnhancedActionEvents|EnhancedInputActionIA_SelectSkill
  (params (ActionValue :type Boolean) (ElapsedSeconds :type Float%20%28double-precision%29) (TriggeredSeconds :type Float%20%28double-precision%29) (InputAction :type Input%20Action%20Object%20Reference :default "/Game/Input/Combat/IA_SelectSkill.IA_SelectSkill"))
  ;[1 1 1] Select skill
  (bind _returnvalue (Class|FabulaPartyIteratorLibrary|TryGetCurrent (Variables|Default|GetSelfPartyIterator)))
  (Abilities|TryActivateAbilitybyClass _returnvalue (Utilities|GetClass (Default|GetSelectedAction (Variables|Default|GetActionSelector))) true))

(event Input|EnhancedActionEvents|EnhancedInputActionIA_PrevTarget
  (params (ActionValue :type Boolean) (ElapsedSeconds :type Float%20%28double-precision%29) (TriggeredSeconds :type Float%20%28double-precision%29) (InputAction :type Input%20Action%20Object%20Reference :default "/Game/Input/Combat/IA_PrevTarget.IA_PrevTarget"))
  (Variables|Default|SetSelectedTargetID (Math|Integer|Clamp(Integer) (+ (Variables|Default|GetSelectedTargetID) -1) 0 (- (Utilities|Array|Length (Variables|Default|GetEnemies)) 1)))
  (CallFunction|RotateActiveTowardsTarget))

(event Input|EnhancedActionEvents|EnhancedInputActionIA_NextTarget
  (params (ActionValue :type Boolean) (ElapsedSeconds :type Float%20%28double-precision%29) (TriggeredSeconds :type Float%20%28double-precision%29) (InputAction :type Input%20Action%20Object%20Reference :default "/Game/Input/Combat/IA_NextTarget.IA_NextTarget"))
  (Variables|Default|SetSelectedTargetID (Math|Integer|Clamp(Integer) (+ (Variables|Default|GetSelectedTargetID) 1) 0 (- (Utilities|Array|Length (Variables|Default|GetEnemies)) 1)))
  (CallFunction|RotateActiveTowardsTarget))

(event Input|EnhancedActionEvents|EnhancedInputActionIA_SelectTarget
  (params (ActionValue :type Boolean) (ElapsedSeconds :type Float%20%28double-precision%29) (TriggeredSeconds :type Float%20%28double-precision%29) (InputAction :type Input%20Action%20Object%20Reference :default "/Game/Input/Combat/IA_SelectTarget.IA_SelectTarget"))
  (Class|FabulaFunctionLibrary|SendTargetReadyCallback (Variables|Default|GetTargettingCallbackAddress) (Utilities|Array|MakeArray (Utilities|Array|Get(acopy) (Variables|Default|GetEnemies) (Variables|Default|GetSelectedTargetID))))
  (bind _returnvalue (Class|FabulaPartyIteratorLibrary|TryGetCurrent (Variables|Default|GetSelfPartyIterator)))
  (Default|CallOnTargettingModeDeactivated _returnvalue))

(event EventBeginPlay)

(event Collision|EventActorBeginOverlap
  (params (OtherActor :type Actor%20Object%20Reference)))

(event EventSelectTargets
  (params (InParams :type Targeting%20Params%20Structure%20%28by%20ref%29) (InCallbackAddress :type Targeting%20Callback%20Address%20Structure))
  (bind _cachedplayercontroller (Variables|Default|GetCachedPlayerController))
  (bind _returnvalue (PlayerController|LocalPlayerSubsystems|GetEnhancedInputLocalPlayerSubsystem _cachedplayercontroller))
  (switch Utilities|FlowControl|Switch|SwitchonETargetType (.PrimaryTargets (Utilities|Struct|BreakTargetingParams InParams))
    (:ETT_Self
      (bind _output_get (Variables|Default|SetTargettingCallbackAddress InCallbackAddress))
      (bind _returnvalue_2 (Class|FabulaPartyIteratorLibrary|TryGetCurrent (Variables|Default|GetSelfPartyIterator)))
      (Class|FabulaFunctionLibrary|SendTargetReadyCallback _output_get (Utilities|Array|MakeArray _returnvalue_2)))
    (:ETT_Enemy
      (Variables|Default|SetTargettingCallbackAddress InCallbackAddress)
      (Default|OpenTargetSelection (Variables|Default|GetCombatMenu))
      (Class|EnhancedInputSubsystemInterface|ClearAllMappings _returnvalue)
      (Input|AddMappingContext _returnvalue "/Game/Input/Combat/IMC_TargetSelect.IMC_TargetSelect" 0 "(bIgnoreAllPressedKeysUntilRelease=True,bForceImmediately=False,bNotifyUserSettings=False)")
      (bind _returnvalue_3 (Class|FabulaPartyIteratorLibrary|TryGetCurrent (Variables|Default|GetSelfPartyIterator)))
      (Default|CallOnTargettingModeActivated _returnvalue_3)
      (bind _returnvalue_4 (Class|FabulaPartyIteratorLibrary|TryGetCurrent (Variables|Default|GetSelfPartyIterator)))
      (bind _returnvalue_5 (Class|FabulaCombatSubsystem|GetOpposingParty (Subsystems|GetFabulaCombatSubsystem) _returnvalue_4))
      (Variables|Default|SetEnemies (Class|FabulaParty|GetAllCreatures _returnvalue_5))
      (Variables|Default|SetSelectedTargetID 0)
      (CallFunction|RotateActiveTowardsTarget))))

(event EventPossessed
  (params (NewController :type Controller%20Object%20Reference))
  (bind _asbp_jrpgplayer_controller (Utilities|Casting|CastToBP_JRPGPlayerController NewController)
    (:then
      (Variables|Default|SetCachedPlayerController _asbp_jrpgplayer_controller)
      (CallFunction|StartCombat))
    (:CastFailed
      (Development|PrintString "BP_CombatPawn possessed by wrong Controller.. It should never happen." true true "(R=1.000000,G=0.000000,B=0.000000,A=1.000000)"))))

(event EventTick
  (params (DeltaSeconds :type Float%20%28single-precision%29)))

(event EventStartTurn
  (bind _cachedplayercontroller (Variables|Default|GetCachedPlayerController))
  (bind _returnvalue (PlayerController|LocalPlayerSubsystems|GetEnhancedInputLocalPlayerSubsystem _cachedplayercontroller))
  (Default|OpenSelfSelection (Variables|Default|GetCombatMenu) (Variables|Default|GetPlayerParty))
  (Class|EnhancedInputSubsystemInterface|ClearAllMappings _returnvalue)
  (Input|AddMappingContext _returnvalue "/Game/Input/Combat/IMC_CombatSelectCharacters.IMC_CombatSelectCharacters" 0 "(bIgnoreAllPressedKeysUntilRelease=True,bForceImmediately=False,bNotifyUserSettings=False)")
  (bind _returnvalue_2 (Class|FabulaPartyIteratorLibrary|TryGetCurrent (Variables|Default|GetSelfPartyIterator)))
  (Game|Player|SetViewTargetwithBlend (Variables|Default|GetCachedPlayerController) (Components|GetOwner _returnvalue_2) 0.0 "VTBlend_Linear" 0.0 false))

(fn ConstructionScript)

(fn RotateActiveTowardsTarget
  (bind _returnvalue (Class|FabulaPartyIteratorLibrary|TryGetCurrent (Variables|Default|GetSelfPartyIterator)))
  (Transformation|SetActorRotation (Components|GetOwner _returnvalue) (Math|Rotator|MakeRotator 0.0 0.0 (.Yaw (Math|Rotator|BreakRotator (Math|Rotator|FindLookatRotation (Transformation|GetActorLocation (Components|GetOwner _returnvalue)) (Transformation|GetActorLocation (Components|GetOwner (Utilities|Array|Get(acopy) (Variables|Default|GetEnemies) (Variables|Default|GetSelectedTargetID))))))))))