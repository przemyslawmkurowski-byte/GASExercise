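; BP_JRPGCreature is a creature actor for a JRPG-style round-based combat system built on the Gameplay Ability System.
; On BeginPlay it registers its attributes with a simplified creature card widget, grants the deal-damage ability and binds to HP reaching zero.
; At zero HP it applies a death effect and ragdolls its mesh.
; Each round start applies a turn-reset effect unless the creature has the Dead tag.
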(event OnRoundStarted(AbilitySystemComp)
  (bind _abilitysystemcomp (Variables|Default|GetAbilitySystemComp))
  (if (not (GameplayTags|HasMatchingGameplayTag _abilitysystemcomp "(TagName=\"Fabula.Status.Dead\")"))
    (GameplayEffects|ApplyGameplayEffectToSelf :self _abilitysystemcomp :GameplayEffectClass "/Game/Effects/GE_ResetTurns.GE_ResetTurns_C")))

(event Custom|OnKilled
  (bind _mesh (Variables|Character|GetMesh))
  (GameplayEffects|ApplyGameplayEffectToSelf :self (Variables|Default|GetAbilitySystemComp) :GameplayEffectClass "/Game/Effects/GE_Death.GE_Death_C")
  ;[1 1 1] This one should react to getting tag, not JUST reaching zero HP. Yes, at this point my patience for GAS reached boiling point
  (Physics|SetSimulatePhysics _mesh true)
  (Collision|SetCollisionProfileName _mesh "Ragdoll" true :!class /Script/Engine.PrimitiveComponent))

(event EventBeginPlay
  (Default|RegisterAttributes (.AsWBP%20Creature%20Card%20Simplified (Utilities|Casting|CastToWBP_CreatureCardSimplified (UserInterface|GetWidget (Variables|Default|GetWidget)))) (Variables|Default|GetAttributeSet))
  (GameplayAbilities|GiveAbility (Variables|Default|GetAbilitySystemComp) "/Game/Abilities/GA_DealDamage.GA_DealDamage_C" 0 -1)
  (bind _returnvalue (GameplayAttributes|GetAttributeSet (Variables|Default|GetAbilitySystemComp) "/Script/GASExercise.FabulaAttributeSet"))
  (bind _asfabula_attribute_set (Utilities|Casting|CastToFabulaAttributeSet _returnvalue))
  (EventDispatchers|BindEventtoOnHPReachedZero _asfabula_attribute_set (delegate Custom|OnKilled)))

(event Collision|EventActorBeginOverlap
  (params (OtherActor :type Actor%20Object%20Reference)))

(event EventTick
  (params (DeltaSeconds :type Float%20%28single-precision%29)))

(fn ConstructionScript)