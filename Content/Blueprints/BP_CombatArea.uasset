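; BP_CombatArea is a combat area Blueprint that defines where two opposing parties stand in a fight.
; It holds five position slots per party, exposed as ordered arrays through GetCombatPositionsForParty0 and GetCombatPositionsForParty1.
; The event graph and construction script are empty, so the asset only provides layout data to whatever calls those getters.
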(event EventBeginPlay)

(event Collision|EventActorBeginOverlap
  (params (OtherActor :type Actor%20Object%20Reference)))

(event EventTick
  (params (DeltaSeconds :type Float%20%28single-precision%29)))

(fn ConstructionScript)

(fn GetCombatPositionsforParty0
  (return (Utilities|Array|MakeArray (Variables|Default|GetPosition_0_0) (Variables|Default|GetPosition_0_1) (Variables|Default|GetPosition_0_2) (Variables|Default|GetPosition_0_3) (Variables|Default|GetPosition_0_4))))

(fn GetCombatPositionsforParty1
  (return (Utilities|Array|MakeArray (Variables|Default|GetPosition_1_0) (Variables|Default|GetPosition_1_1) (Variables|Default|GetPosition_1_2) (Variables|Default|GetPosition_1_3) (Variables|Default|GetPosition_1_4))))