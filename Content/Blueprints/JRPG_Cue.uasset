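; JRPG_Cue is an actor that shows a floating, colored text cue, then destroys itself.
; PlayCue sets the text and color, then plays a timeline rate-scaled by the requested floating duration, assuming a one-second track.
; The timeline raises the TextRender's relative Z from a fixed base offset, scaled by the maximum height.
; When it finishes, the actor waits for the post-float delay before destruction.
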(event Custom|PlayCue
  (params (Text :type Text) (Color :type Color%20Structure) (FloatingDuration :type Float%20%28double-precision%29) (PostFloatingDuration :type Float%20%28double-precision%29) (MaxHeight :type Float%20%28double-precision%29))
  (bind _textrender (Variables|Default|GetTextRender))
  (Components|Timeline|SetPlayRate (Variables|Default|GetMainTimeline) (/ 1.0 FloatingDuration))
  (Rendering|Components|TextRender|SetText _textrender Text)
  (Rendering|Components|TextRender|SetTextRenderColor _textrender Color)
  (bind _newtrack_0 (Timeline|MainTimeline PlayFromStart)
    (:Update
      (Transformation|SetRelativeLocation (Variables|Default|GetTextRender) (Math|Vector|MakeVector 0.0 0.0 (+ (* _newtrack_0 MaxHeight) 1e+02)) false false))
    (:Finished
      (Utilities|FlowControl|Delay PostFloatingDuration)
      (Actor|DestroyActor))))

(event EventBeginPlay)

(event Collision|EventActorBeginOverlap
  (params (OtherActor :type Actor%20Object%20Reference)))

(event EventTick
  (params (DeltaSeconds :type Float%20%28single-precision%29)))

(fn ConstructionScript)