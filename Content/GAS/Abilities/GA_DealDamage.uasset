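; GA_DealDamage is a turn-based combat attack ability: it waits for target selection, commits cost, activates the creature and plays the attack montage.
; When the montage completes, a two-attribute accuracy roll decides each target's outcome: critical success hits, fumble misses, normal rolls compare against the to-hit difficulty.
; Hits apply calculated physical damage through a SetByCaller GE_Damage effect, and both outcomes spawn floating text cues before the turn ends.
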(event Custom|DealDamage
  (params (TargetToHit :type Fabula%20Ability%20System%20Component%20Object%20Reference) (HR :type Integer))
  (bind _finaldamage (CallFunction|CalculateDamage (Math|Conversions|ToFloat(Integer) HR) (Ability|GetAbilitySystemComponent (Ability|GetOwningActorfromActorInfo)) "(AttributeName=\"PrimaryWeaponDamage\",Attribute=/Script/GASExercise.FabulaAttributeSet:PrimaryWeaponDamage,AttributeOwner=\"/Script/CoreUObject.Class'/Script/GASExercise.FabulaAttributeSet'\")" "(TagName=\"Fabula.DamageType.Phys\")" TargetToHit))
  (bind _returnvalue (Ability|GameplayEffect|AssignTagSetbyCallerMagnitude (Ability|MakeOutgoingGameplayEffectSpec "/Game/GAS/GameplayEffects/GE_Damage.GE_Damage_C") "(TagName=\"Fabula.SetByCaller.Damage\")" _finaldamage))
  (GameplayEffects|ApplyGameplayEffectSpecToSelf TargetToHit _returnvalue)
  (CallFunction|PlayBasicCue (CallFunction|GetOwningActorCueTransform TargetToHit) (Utilities|Text|FormatText "{d}" _finaldamage) (Math|Color|MakeColor 0 0 255)))

(event Custom|HandleMiss
  (params (TargetMissed :type Ability%20System%20Component%20Object%20Reference))
  (CallFunction|PlayBasicCue (CallFunction|GetOwningActorCueTransform TargetMissed) "MISS!" (Math|Color|MakeColor 255 255 255)))

(event Ability|EventActivateAbility
  (bind _asfabula_ability_system_component (Utilities|Casting|CastToFabulaAbilitySystemComponent (Ability|GetAbilitySystemComponent (Ability|GetOwningActorfromActorInfo)))
    (:then
      (bind _targets (|FabulaWaitforTarget "None" (Utilities|Struct|MakeTargetingParams _asfabula_ability_system_component "ETT_Enemy" 1 (Variables|Default|GetBaseCost) true) false)
        (:Accepted
          (bind _returnvalue (Ability|CommitAbility))
          (if _returnvalue
            (Class|FabulaAbilitySystemComponent|ActivateCreature (.AsFabula%20Ability%20System%20Component (Utilities|Casting|CastToFabulaAbilitySystemComponent (Ability|GetAbilitySystemComponent (Ability|GetOwningActorfromActorInfo)))))
            (Animation|Montage|PlayMontage (Actor|GetComponentbyClass (Ability|GetAvatarActorfromActorInfo) "/Script/Engine.SkeletalMeshComponent") "/Game/Animations/AM_Attack.AM_Attack"
              (:OnCompleted
                (bind (_outresult _outhighroll) (Class|FabulaHelperLibrary|BasicRoll (Ability|GetAbilitySystemComponent (Ability|GetOwningActorfromActorInfo)) (Variables|Default|GetAccuracyAttribute0) (Variables|Default|GetAccuracyAttribute1))
                  (:None
                    (for _array_element _targets
                      (if (>= _outresult (Variables|Default|GetToHitDifficulty))
                        (CallFunction|DealDamage _array_element _outhighroll)
                        (else
                          (CallFunction|HandleMiss _array_element)))))
                  (:Fumble
                    (for _array_element_2 _targets
                      (CallFunction|HandleMiss _array_element_2)))
                  (:CriticalSuccess
                    (for _array_element_3 _targets
                      (CallFunction|DealDamage _array_element_3 _outhighroll))))
                (Ability|EndAbility)
                (Class|FabulaCombatSubsystem|EndTurn (Subsystems|GetFabulaCombatSubsystem))))
            (else
              (Ability|CancelAbility))))
        (:Cancelled
          (Ability|CancelAbility))))
    (:CastFailed
      (Development|PrintString "Cannot get JRPGAbilitySystemComponent")
      (Ability|CancelAbility))))

(event Ability|EventOnEndAbility
  (params (bWasCancelled :type Boolean)))

(fn PlayBasicCue
  (params (FirstTransform :type Transform) (Text :type Text) (Color :type Color%20Structure))
  (bind _returnvalue (Game|SpawnActorfromClass "/Game/Blueprints/JRPG_Cue.JRPG_Cue_C" FirstTransform "Undefined" "MultiplyWithRoot" 0 0))
  (Default|PlayCue _returnvalue Text Color 0.3 0.2 8e+01))

(fn GetOwningActorCueTransform
  (params (AbilityComponent :type Ability%20System%20Component%20Object%20Reference))
  (return (Transformation|GetActorTransform (Components|GetOwner AbilityComponent))))