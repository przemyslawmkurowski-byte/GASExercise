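; NPC combat controller that plays turns for AI creatures through the Fabula combat subsystem with simple placeholder-style logic.
; On turn start it takes the first creature available for activation and tries to activate that creature's first ability.
; When targets are requested, it picks one random entry from the available targets of the preferred type and returns it through the target-ready callback.
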(event EventBeginPlay)

(event Collision|EventActorBeginOverlap
  (params (OtherActor :type Actor%20Object%20Reference)))

(event EventTick
  (params (DeltaSeconds :type Float%20%28single-precision%29)))

(event EventStartTurn
  (bind _returnvalue (Class|FabulaCombatSubsystem|GetCreaturesAvailableforActivation (Subsystems|GetFabulaCombatSubsystem) self))
  (if (> (Utilities|Array|Length _returnvalue) 0)
    (bind _output_get (Variables|Default|SetSelectedCreature (Utilities|Array|Get(acopy) _returnvalue)))
    (bind _outabilityhandles (Class|AbilitySystemComponent|GetAllAbilities _output_get))
    (Class|AbilitySystemComponent|TryActivateAbility _output_get (Utilities|Array|Get(acopy) _outabilityhandles) true)))

(event EventSelectTargets
  (params (InParams :type Targeting%20Params%20Structure%20%28by%20ref%29) (InCallbackAddress :type Targeting%20Callback%20Address%20Structure))
  (bind (_source _preferredtargets) (Utilities|Struct|BreakTargetingParams InParams))
  (bind _returnvalue (Class|FabulaHelperLibrary|GetAvailableTargets (Subsystems|GetFabulaCombatSubsystem) _source _preferredtargets false))
  (Class|FabulaFunctionLibrary|SendTargetReadyCallback InCallbackAddress (Utilities|Array|MakeArray (Utilities|Array|Get(acopy) _returnvalue (Math|Random|RandomIntegerinRange 0 (- (Utilities|Array|Length _returnvalue) 1))))))

(fn ConstructionScript)